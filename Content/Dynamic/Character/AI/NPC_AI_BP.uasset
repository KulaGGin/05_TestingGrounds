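; NPC AI controller that runs a guard behavior tree with patrol blackboard data and reacts to perceived actors.
; On begin play it sets up the blackboard and tree.
; Perception updates for actors not tagged "Enemy" write the sensed actor to the enemy key and switch on the controlled character's aiming and shooting.
; Losing such an actor clears the key and switches both off.
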(event OnTargetPerceptionUpdated(AIPerception)
  (params (Actor :type Actor%20Object%20Reference) (Stimulus :type AI%20Stimulus%20Structure))
  (if (not (Actor|ActorHasTag Actor "Enemy"))
    (if (.bSuccessfullySensed (Utilities|Struct|BreakAIStimulus Stimulus))
      (AI|Components|Blackboard|SetValueasObject (Variables|Default|GetBlackboardComp) (Variables|Default|GetEnemyKey) Actor)
      (bind _astp_character (Utilities|Casting|CastToCharacter (Pawn|GetControlledPawn)))
      (Variables|/Game/Dynamic/Character/Behavior/Character.Character_C|SetAiming _astp_character true)
      (Variables|/Game/Dynamic/Character/Behavior/Character.Character_C|SetShooting _astp_character true)
      (else
        (AI|Components|Blackboard|ClearValue (Variables|Default|GetBlackboardComp) (Variables|Default|GetEnemyKey))
        (bind _astp_character_2 (Utilities|Casting|CastToCharacter (Pawn|GetControlledPawn)))
        (Variables|/Game/Dynamic/Character/Behavior/Character.Character_C|SetAiming _astp_character_2 false)
        (Variables|/Game/Dynamic/Character/Behavior/Character.Character_C|SetShooting _astp_character_2 false)))))

(event EventBeginPlay
  (bind _blackboardcomponent (Class|AIController|UseBlackboard "/Game/Dynamic/Character/AI/PatrolData.PatrolData"))
  (AI|RunBehaviorTree "/Game/Dynamic/Character/AI/GuardBehavior.GuardBehavior")
  (Variables|Default|SetBlackboardComp _blackboardcomponent))

(fn ConstructionScript)